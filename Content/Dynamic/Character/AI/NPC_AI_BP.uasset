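; AI controller for guard NPCs that detects and engages targets through AI perception and a behavior tree.
; BeginPlay loads the patrol blackboard, seeds its Enemy key with the player pawn and runs GuardBehaviour.
; Perception updates set Enemy to sensed actors lacking the IsEnemy tag and clear it when sensing fails.
; Every tick, the controlled TPCharacter's Aiming and Shooting flags mirror whether a focus actor exists.
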(event OnTargetPerceptionUpdated(AIPerception)
  (params (Actor :type Actor%20Object%20Reference) (Stimulus :type AI%20Stimulus%20Structure))
  (if (not (Actor|ActorHasTag Actor "IsEnemy"))
    (if (.bSuccessfullySensed (Utilities|Struct|BreakAIStimulus Stimulus))
      (AI|Components|Blackboard|SetValueasObject (Variables|Default|GetLocalBlackboard) (Variables|Default|GetEnemy) Actor)
      (else
        (AI|Components|Blackboard|ClearValue (Variables|Default|GetLocalBlackboard) (Variables|Default|GetEnemy))))))

(event EventBeginPlay
  (bind _blackboardcomponent (Class|AIController|UseBlackboard "/Game/Dynamic/Character/AI/PatrolBlackboard.PatrolBlackboard"))
  (Variables|Default|SetLocalBlackboard _blackboardcomponent)
  (AI|Components|Blackboard|SetValueasObject (Variables|Default|GetLocalBlackboard) (Variables|Default|GetEnemy) (Game|Player|GetPlayerPawn 0))
  (AI|RunBehaviorTree "/Game/Dynamic/Character/AI/GuardBehaviour.GuardBehaviour"))

(event EventTick
  (params (DeltaSeconds :type Float%20%28single-precision%29))
  (bind _returnvalue (Class|AIController|GetFocusActor))
  (bind _returnvalue_2 (Utilities|IsValid _returnvalue))
  (bind _astpcharacter (Utilities|Casting|CastToTPCharacter (Pawn|GetControlledPawn)))
  (Variables|/Game/Dynamic/Character/TPCharacter.TPCharacter_C|SetAiming _astpcharacter _returnvalue_2)
  (Variables|/Game/Dynamic/Character/TPCharacter.TPCharacter_C|SetShooting _astpcharacter _returnvalue_2))

(fn ConstructionScript)

(fn PrintSenseInformation
  (params (Stimulus :type AI%20Stimulus%20Structure%20%28by%20ref%29) (object :type Object%20Object%20Reference) (InBool :type Boolean))
  (bind _returnvalue (Class|AIPerceptionSystem|GetSenseClassforStimulus Stimulus))
  (Development|PrintText (Utilities|Text|ToText(String) (Utilities|String|Append (Utilities|GetObjectName (Pawn|GetControlledPawn)) "   " (Utilities|GetClassDisplayName _returnvalue) "   " (Utilities|GetObjectName object) "   Success: " (Utilities|String|ToString(Boolean) InBool)))))