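; Infinite terrain tile that scatters containers, boxes and rocks on BeginPlay through PlaceActors.
; When the player exits its locking volume nearer the next tile's marker, it locks its bounding wall (red), unlocks the next (green) and has the game mode spawn another tile.
; Tiles form a doubly linked chain; player overlap with the destroy volume clears neighbour links and destroys the tile.
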(event OnComponentEndOverlap(LockingVolume)
  (params (OverlappedComponent :type Primitive%20Component%20Object%20Reference) (OtherActor :type Actor%20Object%20Reference) (OtherComp :type Primitive%20Component%20Object%20Reference) (OtherBodyIndex :type Integer))
  (bind _nexttile (Variables|Default|GetNextTile))
  (Utilities|IfPlayerExecute OtherActor)
  (Utilities|IfProgressedExecute OtherActor)
  (CallFunction|Lock)
  (Utilities|IsValid _nexttile
    (:Is%20Valid
      (CallFunction|Unlock _nexttile)
      (bind _asinfinite_terrain_game_mode (Utilities|Casting|CastToInfiniteTerrainGameMode (Game|GetGameMode)))
      (Default|SpawnTile _asinfinite_terrain_game_mode true))))

(event OnComponentBeginOverlap(DestroyVolume)
  (params (OverlappedComponent :type Primitive%20Component%20Object%20Reference) (OtherActor :type Actor%20Object%20Reference) (OtherComp :type Primitive%20Component%20Object%20Reference) (OtherBodyIndex :type Integer) (bFromSweep :type Boolean) (SweepResult :type Hit%20Result%20Structure%20%28by%20ref%29))
  (Utilities|IfPlayerExecute OtherActor)
  (CallFunction|CleanUpandDelete))

(event EventBeginPlay
  (Class|Tile|PlaceActors "/Game/Dynamic/Terrain/Props/BP_Container.BP_Container_C" 1 3)
  (Class|Tile|PlaceActors "/Game/Dynamic/Terrain/Props/BP_Box.BP_Box_C" 2 4)
  (Class|Tile|PlaceActors "/Game/Dynamic/Terrain/Props/BP_Rock1.BP_Rock1_C" 1 10))

(fn ConstructionScript)

(fn GetAttachLocation
  (return (Transformation|GetWorldTransform (Variables|Default|GetArrow))))

(fn Unlock
  (Collision|SetCollisionEnabled (Variables|Default|GetBoundingWall) "NoCollision")
  (Rendering|Material|SetMaterial (Variables|Default|GetBoundingWall) 0 "/Game/Dynamic/Terrain/MI_Barrier_Green.MI_Barrier_Green"))

(fn Lock
  (Collision|SetCollisionEnabled (Variables|Default|GetBoundingWall) "QueryAndPhysics")
  (Rendering|Material|SetMaterial (Variables|Default|GetBoundingWall) 0 "/Game/Dynamic/Terrain/MI_Barrier_Red.MI_Barrier_Red"))

(fn PrintTile
  (params (A :type String) (Object :type Object%20Object%20Reference))
  (Development|PrintString (Utilities|String|Append A (Utilities|GetDisplayName Object))))

(fn DistancetoBounds
  (params (Actor :type Actor%20Object%20Reference))
  (return (Math|Vector|VectorLength (- (Transformation|GetWorldLocation (Variables|Default|GetMarker)) (Transformation|GetActorLocation Actor)))))

(fn PrintDistancetoBounds
  (params (InFloat :type Float%20%28single-precision%29) (Text :type String))
  (Development|PrintString (Utilities|String|Append Text (Utilities|String|ToString(Float) InFloat))))

(fn ClearPreviousTileNext
  (bind _previoustile (Variables|Default|GetPreviousTile))
  (Utilities|IsValid _previoustile
    (:Is%20Valid
      (Variables|BP_Tile_C|SetNextTile _previoustile 0))))

(fn ClearNextTilePrevious
  (bind _nexttile (Variables|Default|GetNextTile))
  (Utilities|IsValid _nexttile
    (:Is%20Valid
      (Variables|BP_Tile_C|SetPreviousTile _nexttile 0))))

(fn CleanUpandDelete
  (CallFunction|ClearPreviousTileNext)
  (CallFunction|ClearNextTilePrevious)
  (Actor|DestroyActor))

(fn NextMinusPrevious
  (params (Actor :type Actor%20Object%20Reference))
  (bind _distance (CallFunction|DistancetoBounds Actor))
  (CallFunction|PrintDistancetoBounds _distance "Distance to this ")
  (bind _distance_2 (CallFunction|DistancetoBounds (Variables|Default|GetNextTile) Actor))
  (CallFunction|PrintDistancetoBounds _distance_2 "Distance to next ")
  (return (- _distance_2 _distance)))